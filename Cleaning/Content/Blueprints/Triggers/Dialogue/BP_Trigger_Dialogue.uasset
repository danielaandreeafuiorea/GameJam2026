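; One-shot trigger actor that starts a dialogue sequence when a player character overlaps it.
; It casts the overlapping actor to both the first-person character and BP_Player, calling StartDialogue on whichever matches.
; The trigger's line and speaker lists, optional voice playback and optional level transition settings are passed to the player, which handles the dialogue.
; An IsConsumed flag, set after a successful call, blocks repeat triggering.
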(event Collision|EventActorBeginOverlap
  (params (OtherActor :type Actor%20Object%20Reference))
  (if (not (Variables|Default|GetIsConsumed))
    (Utilities|FlowControl|Sequence
      (:then_0
        (bind _asbp_player_char_first_person (Utilities|Casting|CastToBP_PlayerCHAR_FirstPerson OtherActor))
        (bind _output_get (Variables|Default|SetFP%20Player _asbp_player_char_first_person))
        (Default|StartDialogue _output_get (Variables|Default|GetLine%20List) (Variables|Default|GetSpeaker%20List) (Variables|Default|GetLoadLevel) (Variables|Default|GetLevelToLoad) (Variables|Default|GetLevelTransitionLength) (Variables|Default|GetLevelTransitionSFX) (Variables|Default|GetPlayVoiceSFX) (Variables|Default|GetVoiceToPlay)))
      (:then_1
        (bind _asbp_player (Utilities|Casting|CastToBP_Player OtherActor))
        (bind _output_get_2 (Variables|Default|SetTD%20Player _asbp_player))
        (Default|StartDialogue _output_get_2 (Variables|Default|GetLine%20List) (Variables|Default|GetSpeaker%20List) (Variables|Default|GetLoadLevel) (Variables|Default|GetLevelToLoad) (Variables|Default|GetLevelTransitionLength) (Variables|Default|GetLevelTransitionSFX) (Variables|Default|GetPlayVoiceSFX) (Variables|Default|GetVoiceToPlay))))
    (Variables|Default|SetIsConsumed true)))

(fn ConstructionScript)