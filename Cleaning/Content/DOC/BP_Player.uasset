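; Player character Blueprint for a top-down mopping game, with sprite movement, cleaning, shooting, poking, interaction and knockback with a red damage flash.
; While cleaning, Tick stamps water marks through the water trail manager every step distance, cleans overlapped blood puddles and drains mop water, warning when empty until refilled.
; Water projectiles aim at the cursor; pokes hit the nearby enemy or close skeletons.
; It also creates the task and dialogue HUDs and picks opening dialogue by level name.
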(event Custom|RefillWarningMessage
  (bind _returnvalue (UserInterface|CreateWidget "/Game/DOC/BloodPuddleLogic/W_RefillWaterMessage.W_RefillWaterMessage_C" (Game|GetPlayerController 0)))
  (bind _output_get (Variables|Default|SetWarningMessageWidget _returnvalue))
  (UserInterface|Viewport|AddtoViewport _output_get 0))

(event Custom|StopWarningMessage
  (bind _warningmessagewidget (Variables|Default|GetWarningMessageWidget))
  (Utilities|IsValid _warningmessagewidget
    (:Is%20Valid
      (Default|StopAnim _warningmessagewidget))))

(event Custom|GetDamaged
  (params (DamageSource :type BP%20Enemy%20Object%20Reference))
  (Character|LaunchCharacter (* (Class|KismetMathLibrary|VectorNormal2D (- (Transformation|GetActorLocation) (Transformation|GetActorLocation DamageSource)) 0.0001) (Variables|Default|GetKnockBackStrength)) true false)
  (Sprite|SetSpriteColor (Variables|Default|GetPlayerSprite) "(R=1.000000,G=0.011477,B=0.000000,A=1.000000)")
  (Utilities|FlowControl|Delay 0.2)
  (Sprite|SetSpriteColor (Variables|Default|GetPlayerSprite) "(R=1.000000,G=1.000000,B=1.000000,A=1.000000)"))

(event Custom|SetIsPoking
  (Variables|Default|SetisPoking false))

(event Custom|Start%20Opening%20Dialogue
  (bind _returnvalue (Game|GetCurrentLevelName true))
  (bind _output_get (Variables|Default|SetCurrentLevelName _returnvalue))
  (if (Utilities|Enum|Equal(Enum) _output_get "TestMapDOC")
    (Default|StartSpeaking (Variables|Default|GetDialogueHUD) (Variables|OpeningLines|GetDay1LineList) (Variables|OpeningLines|GetDay1SpeakerList) false "None" 0.0 0 false)
    (elif (Utilities|Enum|Equal(Enum) (Variables|Default|GetCurrentLevelName) "Day2")
      (Default|StartSpeaking (Variables|Default|GetDialogueHUD) (Variables|OpeningLines|GetDay2LineList) (Variables|OpeningLines|GetDay2SpeakerList) false "None" 0.0 0 false)
      (elif (Utilities|Enum|Equal(Enum) (Variables|Default|GetCurrentLevelName) "Day3")
        (Default|StartSpeaking (Variables|Default|GetDialogueHUD) (Variables|OpeningLines|GetDay3LineList) (Variables|OpeningLines|GetDay3SpeakerList) false "None" 0.0 0 false)
        (elif (Utilities|Enum|Equal(Enum) (Variables|Default|GetCurrentLevelName) "BossBattle")
          (Default|StartSpeaking (Variables|Default|GetDialogueHUD) (Variables|OpeningLines|GetDay4LineList) (Variables|OpeningLines|GetDay4SpeakerList) false "None" 0.0 0 false))))))

(event Input|EnhancedActionEvents|EnhancedInputActionIA_Move
  (params (ActionValue :type Vector%202D%20Structure) (ElapsedSeconds :type Float%20%28double-precision%29) (TriggeredSeconds :type Float%20%28double-precision%29) (InputAction :type Input%20Action%20Object%20Reference :default "/Game/DOC/IA_Move.IA_Move"))
  (bind (_x _y) (Math|Vector2D|BreakVector2D ActionValue))
  (Pawn|Input|AddMovementInput (Math|Vector|Normalize (Math|Vector|MakeVector _x _y 0.0)) 1.0 false)
  (if (> _y 0.0)
    (Transformation|SetRelativeRotation (Variables|Default|GetPlayerSprite) "0.000000,90.000000,0.000000" false false)
    (else
      (Transformation|SetRelativeRotation (Variables|Default|GetPlayerSprite) "0.000000,-90.000000,0.000000" false false))))

(event Input|EnhancedActionEvents|EnhancedInputActionIA_Clean
  (params (ActionValue :type Boolean) (ElapsedSeconds :type Float%20%28double-precision%29) (TriggeredSeconds :type Float%20%28double-precision%29) (InputAction :type Input%20Action%20Object%20Reference :default "/Game/DOC/IA_Clean.IA_Clean"))
  (:Started
    (Variables|Default|SetisCleaning true)
    (Variables|Default|SetLastCleanLocation (Transformation|GetWorldLocation (Variables|Default|GetMopPoint))))
  (:Canceled
    (Variables|Default|SetisCleaning false :!label _label)
    (Variables|Default|SetisMopping false))
  (:Completed
    (goto _label)))

(event Input|EnhancedActionEvents|EnhancedInputActionIA_Poke
  (params (ActionValue :type Boolean) (ElapsedSeconds :type Float%20%28double-precision%29) (TriggeredSeconds :type Float%20%28double-precision%29) (InputAction :type Input%20Action%20Object%20Reference :default "/Game/DOC/IA_Poke.IA_Poke"))
  (bind _nearbyenemy (Variables|Default|GetNearbyEnemy))
  (:Started
    (if (not (Variables|Default|GetisMopping))
      (Variables|Default|SetisPoking true)
      (Utilities|Time|SetTimerbyEvent (delegate Custom|SetIsPoking) 0.1)
      (Utilities|IsValid _nearbyenemy
        (:Is%20Valid
          (Default|GetPoked _nearbyenemy))
        (:Is%20Not%20Valid
          (bind _outactors (Actor|GetAllActorsOfClass "/Game/AI/B_Skelly.B_Skelly_C"))
          (for _array_element _outactors
            (if (< (Math|Vector|Distance(Vector) (Transformation|GetActorLocation _array_element) (Transformation|GetActorLocation)) 1.5e+02)
              (Default|Poke _array_element))))))))

(event Input|EnhancedActionEvents|EnhancedInputActionIA_Shoot
  (params (ActionValue :type Boolean) (ElapsedSeconds :type Float%20%28double-precision%29) (TriggeredSeconds :type Float%20%28double-precision%29) (InputAction :type Input%20Action%20Object%20Reference :default "/Game/DOC/IA_Shoot.IA_Shoot"))
  (bind _playersprite (Variables|Default|GetPlayerSprite))
  (bind _returnvalue (Transformation|GetWorldLocation _playersprite))
  (bind (_x _y) (Math|Vector|BreakVector _returnvalue))
  (:Started
    (if (not (Variables|Default|GetisMopping))
      (Game|SpawnActorfromClass "/Game/AI/B_WaterProjectile.B_WaterProjectile_C" (Math|Transform|MakeTransform (Math|Vector|MakeVector _x _y 1e+02) (Math|Rotator|MakeRotator 0.0 0.0 (.yaw (Math|Rotator|FindLookatRotation _returnvalue (.ImpactPoint (Collision|BreakHitResult (.HitResult (Game|Player|GetHitResultUnderCursorbyChannel (Game|GetPlayerController 0) "TraceTypeQuery1" true))))))) "1.000000,1.000000,1.000000") "Undefined" "MultiplyWithRoot" 0 0))))

(event Input|EnhancedActionEvents|EnhancedInputActionIA_Interact
  (params (ActionValue :type Boolean) (ElapsedSeconds :type Float%20%28double-precision%29) (TriggeredSeconds :type Float%20%28double-precision%29) (InputAction :type Input%20Action%20Object%20Reference :default "/Game/DOC/IA_Interact.IA_Interact"))
  (bind _currentinteractable (Variables|Default|GetCurrentInteractable))
  (bind _nearbyenemy (Variables|Default|GetNearbyEnemy))
  (:Started
    (Utilities|IsValid _nearbyenemy
      (:Is%20Valid
        (Default|Interact _nearbyenemy))
      (:Is%20Not%20Valid
        (Utilities|IsValid _currentinteractable
          (:Is%20Valid
            (Default|Interact _currentinteractable self)))))))

(event EventBeginPlay
  (Variables|/Script/Engine.PlayerController|SetbShowMouseCursor (Game|GetPlayerController 0) true)
  (Input|AddMappingContext (PlayerController|LocalPlayerSubsystems|GetEnhancedInputLocalPlayerSubsystem (Game|GetPlayerController 0)) "/Game/DOC/IMC_Player.IMC_Player" 0 "(bIgnoreAllPressedKeysUntilRelease=True,bForceImmediately=False,bNotifyUserSettings=False)")
  (bind _returnvalue (Actor|GetActorOfClass "/Game/DOC/BloodPuddleLogic/B_WaterTrailManager.B_WaterTrailManager_C"))
  (Variables|Default|SetWaterTrailManager _returnvalue)
  (Variables|Default|SetCurrentMopWater (Variables|Default|GetMaxMopWater))
  (bind _returnvalue_2 (UserInterface|CreateWidget "/Game/UI/WB_TaskList.WB_TaskList_C"))
  (bind _output_get (Variables|Default|SetWidgetTaskList _returnvalue_2))
  (UserInterface|Viewport|AddtoViewport _output_get 0)
  (bind _returnvalue_3 (UserInterface|CreateWidget "/Game/Blueprints/WidgetBlueprints/HUD/WBP_Dialogue_HUD.WBP_Dialogue_HUD_C"))
  (bind _output_get_2 (Variables|Default|SetDialogueHUD _returnvalue_3))
  (UserInterface|Viewport|AddtoViewport _output_get_2 0))

(event Collision|EventActorBeginOverlap
  (params (OtherActor :type Actor%20Object%20Reference)))

(event EventTick
  (params (DeltaSeconds :type Float%20%28single-precision%29))
  (bind _moppoint (Variables|Default|GetMopPoint))
  (bind _returnvalue (Transformation|GetWorldLocation _moppoint))
  (if (Variables|Default|GetisCleaning)
    (if (not (Variables|Default|GetisInTransition))
      (bind _output_get (Variables|Default|SetDistanceMoved (Math|Vector|Distance2D(Vector) (Transformation|GetWorldLocation (Variables|Default|GetMopPoint)) (Variables|Default|GetLastCleanLocation))))
      (if (>= _output_get (Variables|Default|GetCleanStepDistance))
        (if (> (Variables|Default|GetCurrentMopWater) 0.0)
          (Variables|Default|SetisMopping true)
          (Default|AddWaterMark (Variables|Default|GetWaterTrailManager) (Transformation|GetWorldLocation (Variables|Default|GetMopPoint)) (Variables|Default|GetMopWidth))
          (bind _outactors (Collision|SphereOverlapActors (Transformation|GetWorldLocation (Variables|Default|GetMopPoint)) 1e+01 (Utilities|Array|MakeArray "ObjectTypeQuery2") "/Game/DOC/BloodPuddleLogic/BP_BloodPuddle.BP_BloodPuddle_C"))
          (for _array_element _outactors
            (bind _asbp_blood_puddle (Utilities|Casting|CastToBP_BloodPuddle _array_element))
            (Default|Clean _asbp_blood_puddle _returnvalue (Variables|Default|GetMopWidth)))
          (Variables|Default|SetLastCleanLocation _returnvalue)
          (CallFunction|ConsumeMopWater (Variables|Default|GetDistanceMoved))
          (else
            (Variables|Default|SetLastCleanLocation (Transformation|GetWorldLocation (Variables|Default|GetMopPoint)))
            (Variables|Default|SetisMopping false))))
      (else
        (Variables|Default|SetisMopping false :!label _label)))
    (else
      (goto _label))))

(event Input|KeyboardEvents|DebugKeyO
  (params (Key :type Key%20Structure :default "None") (ActionValue :type Input%20Action%20Value%20Structure)))

(fn ConstructionScript)

(fn ConsumeMopWater
  (params (DistanceMoved :type Float%20%28double-precision%29))
  (bind _output_get (Variables|Default|SetCurrentMopWater (Math|Float|Clamp(Float) (- (Variables|Default|GetCurrentMopWater) (* DistanceMoved (Variables|Default|GetWaterDrainPerCm))) 0.0 (Variables|Default|GetMaxMopWater))))
  (if (<= _output_get 0.0)
    (CallFunction|RefillWarningMessage)))

(fn RefillWater
  (Variables|Default|SetCurrentMopWater (Variables|Default|GetMaxMopWater))
  (CallFunction|StopWarningMessage))