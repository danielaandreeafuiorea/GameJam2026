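; Phased enemy AI character with a flipbook sprite that hunts the player and opens widget minigames on interaction.
; Phase 1 makes damaging straight navmesh runs, periodically re-aimed and bouncing on arrival, until timed B_WaterTrailManager checks make it slip, enabling interaction.
; Finishing that minigame sends it to a TargetPoint for phase 2, which still damages.
; Completing the second starts phase 3: a timer-driven chase interruptible by poke knockback.
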(event OnComponentBeginOverlap(CapsuleComponent)
  (params (OverlappedComponent :type Primitive%20Component%20Object%20Reference) (OtherActor :type Actor%20Object%20Reference) (OtherComp :type Primitive%20Component%20Object%20Reference) (OtherBodyIndex :type Integer) (bFromSweep :type Boolean) (SweepResult :type Hit%20Result%20Structure%20%28by%20ref%29))
  (bind _asbp_player (Utilities|Casting|CastToBP_Player OtherActor))
  (if (and (== (Variables|Default|GetEnemyPhase) 1) (not (Variables|Default|GetisSlipping)))
    (Default|GetDamaged _asbp_player self :!label _label)
    (elif (== (Variables|Default|GetEnemyPhase) 2)
      (goto _label))))

(event OnComponentBeginOverlap(InteractionRange)
  (params (OverlappedComponent :type Primitive%20Component%20Object%20Reference) (OtherActor :type Actor%20Object%20Reference) (OtherComp :type Primitive%20Component%20Object%20Reference) (OtherBodyIndex :type Integer) (bFromSweep :type Boolean) (SweepResult :type Hit%20Result%20Structure%20%28by%20ref%29))
  (bind _asbp_player (Utilities|Casting|CastToBP_Player OtherActor))
  (Variables|Default|SetPlayerInInteractionRange true)
  (Variables|Default|SetPlayerReference _asbp_player)
  (Variables|/Game/DOC/BP_Player.BP_Player_C|SetNearbyEnemy _asbp_player self))

(event OnComponentEndOverlap(InteractionRange)
  (params (OverlappedComponent :type Primitive%20Component%20Object%20Reference) (OtherActor :type Actor%20Object%20Reference) (OtherComp :type Primitive%20Component%20Object%20Reference) (OtherBodyIndex :type Integer))
  (bind _asbp_player (Utilities|Casting|CastToBP_Player OtherActor))
  (Variables|Default|SetPlayerInInteractionRange false)
  (Variables|Default|SetPlayerReference 0)
  (Variables|/Game/DOC/BP_Player.BP_Player_C|SetNearbyEnemy _asbp_player 0))

(event Custom|AimAtPlayer
  (Variables|Default|SetCurrentDirection (Class|KismetMathLibrary|VectorNormal2D (- (Transformation|GetActorLocation (Game|GetPlayerCharacter 0)) (Transformation|GetActorLocation)) 0.0001))
  (CallFunction|MoveinCurrentDirection))

(event Custom|FinishedTask
  (Variables|Default|SetEnemyPhase 2)
  (Input|EnableInput (Game|Player|GetPlayerPawn 0) (Game|GetPlayerController 0))
  (Widget|SetVisibility (Variables|Default|GetFirstPhaseMinigame) "Collapsed")
  (Widget|RemovefromParent (Variables|Default|GetFirstPhaseMinigame))
  (Variables|Default|SetFirstPhaseMinigame 0)
  (CallFunction|StartPhase2))

(event Custom|StartMinigame_1
  (Input|DisableInput (Game|Player|GetPlayerPawn 0) (Game|GetPlayerController 0))
  (bind _returnvalue (UserInterface|CreateWidget "/Game/UIMinigames/Playable/W_SwipeBloodHERO.W_SwipeBloodHERO_C"))
  (Variables|Default|SetFirstPhaseMinigame _returnvalue)
  (UserInterface|Viewport|AddtoViewport _returnvalue 0)
  (Variables|/Game/UIMinigames/Playable/W_SwipeBloodHERO.W_SwipeBloodHERO_C|SetisPlayer _returnvalue true)
  (Variables|/Game/UIMinigames/Playable/W_SwipeBloodHERO.W_SwipeBloodHERO_C|SetParentPlayer _returnvalue self))

(event Custom|StartMinigame_2
  (Input|DisableInput (Game|Player|GetPlayerPawn 0) (Game|GetPlayerController 0))
  (bind _returnvalue (UserInterface|CreateWidget "/Game/UIMinigames/Playable/W_ShootCadavresHERO.W_ShootCadavresHERO_C"))
  (bind _output_get (Variables|Default|SetSecondPhaseMinigame _returnvalue))
  (UserInterface|Viewport|AddtoViewport _output_get 0)
  (Variables|/Game/UIMinigames/Playable/W_ShootCadavresHERO.W_ShootCadavresHERO_C|SetisPlayer _returnvalue true)
  (Variables|/Game/UIMinigames/Playable/W_ShootCadavresHERO.W_ShootCadavresHERO_C|SetParentPlayer _returnvalue self))

(event Custom|Finished2Task
  (Variables|Default|SetEnemyPhase 3)
  (Input|EnableInput (Game|Player|GetPlayerPawn 0) (Game|GetPlayerController 0))
  (Widget|SetVisibility (Variables|Default|GetSecondPhaseMinigame) "Collapsed")
  (Widget|RemovefromParent (Variables|Default|GetSecondPhaseMinigame))
  (Variables|Default|SetSecondPhaseMinigame 0)
  (CallFunction|StartPhase3))

(event Custom|StartPhase3
  (Variables|Default|SetisSlipping false)
  (Variables|/Script/Engine.CharacterMovementComponent|SetMaxWalkSpeed (Variables|Character|GetCharacterMovement) 1e+02)
  (Components|Sphere|SetSphereRadius (Variables|Default|GetInteractionRange) 3e+02 true)
  (Utilities|Time|SetTimerbyEvent (delegate Custom|UpdatePhase3Chase) 0.2 true))

(event Custom|UpdatePhase3Chase
  (if (and (== (Variables|Default|GetEnemyPhase) 3) (not (Variables|Default|GetisBeingPushed)))
    (AI|AIMoveTo self (Transformation|GetActorLocation (Game|GetPlayerCharacter 0)) 0 5e+01 true)
    (else
      (Components|Movement|StopMovementImmediately (Variables|Character|GetCharacterMovement)))))

(event Custom|GetPoked
  (Variables|Default|SetisBeingPushed true)
  (Character|LaunchCharacter (* (Class|KismetMathLibrary|VectorNormal2D (- (Transformation|GetActorLocation) (Transformation|GetActorLocation (Game|GetPlayerCharacter 0))) 0.0001) (Variables|Default|GetPokeStrength)) true false)
  (Utilities|FlowControl|Delay 0.35)
  (Variables|Default|SetisBeingPushed false))

(event Custom|Finished3Task)

(event Custom|ChooseBounceDirection
  (Variables|Default|SetCurrentDirection (Class|KismetMathLibrary|VectorNormal2D (Math|Vector|RotateVectorAroundAxis (* (Variables|Default|GetCurrentDirection) -1.0) (Math|Random|RandomFloatinRange -4e+01 4e+01) "0.000000,0.000000,1.000000") 0.0001))
  (CallFunction|MoveinCurrentDirection))

(event Custom|RetargetPlayer
  (if (and (== (Variables|Default|GetEnemyPhase) 1) (not (Variables|Default|GetisSlipping)))
    (AI|Navigation|StopMovement (Pawn|GetController))
    (CallFunction|AimatPlayer)))

(event Custom|CheckForWater
  (if (and (== (Variables|Default|GetEnemyPhase) 1) (not (Variables|Default|GetisSlipping)))
    (bind _returnvalue (Actor|GetActorOfClass "/Game/DOC/BloodPuddleLogic/B_WaterTrailManager.B_WaterTrailManager_C"))
    (bind _iswet (Default|IsLocationWet _returnvalue (Transformation|GetActorLocation) 1e+01))
    (if _iswet
      (CallFunction|StartSlip))))

(event Custom|StartSlip
  (Variables|Default|SetisSlipping true)
  (AI|Navigation|StopMovement (Pawn|GetController))
  (Components|Movement|StopMovementImmediately (Variables|Character|GetCharacterMovement)))

(event Custom|Interact
  (if (and (== (Variables|Default|GetEnemyPhase) 1) (Variables|Default|GetisSlipping))
    (CallFunction|StartMinigame1)
    (elif (== (Variables|Default|GetEnemyPhase) 2)
      (CallFunction|StartMinigame2))))

(event Custom|StartMinigame_3
  (Input|DisableInput (Game|Player|GetPlayerPawn 0) (Game|GetPlayerController 0))
  (bind _returnvalue (UserInterface|CreateWidget "/Game/UIMinigames/Playable/W_CrawlingBugsHERO.W_CrawlingBugsHERO_C"))
  (UserInterface|Viewport|AddtoViewport _returnvalue 0)
  (Variables|/Game/UIMinigames/Playable/W_CrawlingBugsHERO.W_CrawlingBugsHERO_C|SetisPlayer _returnvalue true)
  (Variables|/Game/UIMinigames/Playable/W_CrawlingBugsHERO.W_CrawlingBugsHERO_C|SetParentPlayer _returnvalue self))

(event Custom|MoveInCurrentDirection
  (bind _hitlocation (Class|NavigationSystemV1|NavigationRaycast (Transformation|GetActorLocation) (+ (Transformation|GetActorLocation) (* (Variables|Default|GetCurrentDirection) (Variables|Default|GetTravelDistance))) 0 (Pawn|GetController)))
  (AI|AIMoveTo self _hitlocation 0 3e+01 false
    (:OnSuccess
      (if (and (== (Variables|Default|GetEnemyPhase) 1) (not (Variables|Default|GetisSlipping)))
        (CallFunction|ChooseBounceDirection)))))

(event Custom|StartPhase2
  (Variables|Default|SetisSlipping false)
  (AI|AIMoveTo self (Transformation|GetActorLocation (Variables|Default|GetPhase2Target)) 0 3e+01 false))

(event EventBeginPlay
  (bind _returnvalue (Actor|GetActorOfClass "/Script/Engine.TargetPoint"))
  (Variables|Default|SetPhase2Target _returnvalue)
  (CallFunction|AimatPlayer)
  (Utilities|Time|SetTimerbyEvent (delegate Custom|RetargetPlayer) (Variables|Default|GetRetargetInterval) true)
  (Utilities|Time|SetTimerbyEvent (delegate Custom|CheckForWater) 0.1 true))

(event Collision|EventActorBeginOverlap
  (params (OtherActor :type Actor%20Object%20Reference)))

(event EventTick
  (params (DeltaSeconds :type Float%20%28single-precision%29))
  (Transformation|SetWorldRotation (Variables|Default|GetPaperFlipbook) (Math|Rotator|MakeRotator 0.0 0.0 9e+01) false false))

(fn ConstructionScript)