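; BP_Interactable is a base interactable actor that shows a prompt widget when the player comes within overlap range.
; On BeginPlay it passes InteractionText to its WB_InteractionPrompt widget component and hides it.
; Overlap begin and end set or clear the BP_Player's CurrentInteractable and show or hide the prompt.
; The Interact function takes the player and is left empty, apparently for child Blueprints to override.
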(event EventBeginPlay
  (bind _aswb_interaction_prompt (Utilities|Casting|CastToWB_InteractionPrompt (UserInterface|GetUserWidgetObject (Variables|Default|GetWidget))))
  (Default|SetInteractionText _aswb_interaction_prompt (Variables|Default|GetInteractionText))
  (Widget|SetVisibility _aswb_interaction_prompt "Hidden"))

(event Collision|EventActorBeginOverlap
  (params (OtherActor :type Actor%20Object%20Reference))
  (bind _asbp_player (Utilities|Casting|CastToBP_Player OtherActor))
  (Variables|/Game/DOC/BP_Player.BP_Player_C|SetCurrentInteractable _asbp_player self)
  (bind _aswb_interaction_prompt (Utilities|Casting|CastToWB_InteractionPrompt (UserInterface|GetUserWidgetObject (Variables|Default|GetWidget))))
  (Widget|SetVisibility _aswb_interaction_prompt "Visible"))

(event EventTick
  (params (DeltaSeconds :type Float%20%28single-precision%29)))

(event Collision|EventActorEndOverlap
  (params (OtherActor :type Actor%20Object%20Reference))
  (bind _asbp_player (Utilities|Casting|CastToBP_Player OtherActor))
  (Variables|/Game/DOC/BP_Player.BP_Player_C|SetCurrentInteractable _asbp_player 0)
  (bind _aswb_interaction_prompt (Utilities|Casting|CastToWB_InteractionPrompt (UserInterface|GetUserWidgetObject (Variables|Default|GetWidget))))
  (Widget|SetVisibility _aswb_interaction_prompt "Hidden"))

(fn ConstructionScript)

(fn Interact
  (params (BP_Player :type BP%20Player%20Object%20Reference)))