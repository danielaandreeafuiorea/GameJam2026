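; Blood puddle actor that is mopped away and counts toward the game instance's cleaning tasks.
; Clean maps a world position and mop width to plane UV space and draws a brush into a render-target mask used by the puddle material.
; Every few strokes, it renders remaining blood to a tiny target and sums red pixels against the initial amount.
; Past the threshold, it disables collision, fades out, updates tasks and destroys itself.
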(event Custom|PuddleCleaned
  (Variables|Default|SetisCompleted true)
  (Collision|SetCollisionEnabled (Variables|Default|GetCleaningCollision) "NoCollision")
  (bind _fade (Timeline|FinalFade PlayFromStart)
    (:Update
      (Rendering|Material|SetScalarParameterValue (Variables|Default|GetBloodMaterialDynamic) "FinalFade" _fade :!class /Script/Engine.MaterialInstanceDynamic))
    (:Finished
      (bind _asbp_game_instance (Utilities|Casting|CastToBP_GameInstance (Game|GetGameInstance)))
      (Math|Integer|IncrementInt (Variables|/Game/DOC/BP_GameInstance.BP_GameInstance_C|GetBlood3DCleaned _asbp_game_instance)
        (:%20%20
          (Default|CheckTasks _asbp_game_instance)
          (Default|Update _asbp_game_instance "NewEnumerator0")
          (Actor|DestroyActor))))))

(event EventBeginPlay
  (bind _returnvalue (Rendering|CreateRenderTarget2D 512 512 "RTF_RGBA16f" "(R=1.000000,G=1.000000,B=1.000000,A=1.000000)"))
  (Variables|Default|SetCleanRenderTarget _returnvalue)
  (bind _returnvalue_2 (Rendering|Material|CreateDynamicMaterialInstance (Variables|Default|GetBloodPlane) 0 "/Game/DOC/BloodPuddleLogic/M_BloodPuddle.M_BloodPuddle" "None" :!class /Script/Engine.PrimitiveComponent))
  (Variables|Default|SetBloodMaterialDynamic _returnvalue_2)
  (Rendering|Material|SetTextureParameterValue (Variables|Default|GetBloodMaterialDynamic) "CleanMask" (Variables|Default|GetCleanRenderTarget))
  (bind _returnvalue_3 (Rendering|CreateRenderTarget2D 32 32 "RTF_RGBA8"))
  (Variables|Default|SetProgressRenderTarget _returnvalue_3)
  (bind _returnvalue_4 (Rendering|Material|CreateDynamicMaterialInstance "/Game/DOC/BloodPuddleLogic/M_BloodProgress.M_BloodProgress" "None" "None" :!class /Script/Engine.KismetMaterialLibrary))
  (bind _output_get (Variables|Default|SetBloodProgressMaterialDynamic _returnvalue_4))
  (Rendering|Material|SetTextureParameterValue _output_get "CleanMask" (Variables|Default|GetCleanRenderTarget))
  (bind _boodammount (CallFunction|MeasureBloodAmmount))
  (Variables|Default|SetInitialBloodAmount _boodammount))

(event Collision|EventActorBeginOverlap
  (params (OtherActor :type Actor%20Object%20Reference)))

(event EventTick
  (params (DeltaSeconds :type Float%20%28single-precision%29)))

(fn ConstructionScript)

(fn Clean
  (params (WorldLocation :type Vector) (MopWidth :type Float%20%28double-precision%29))
  (bind _bloodplane (Variables|Default|GetBloodPlane))
  (bind _bloodplane_2 (Variables|Default|GetBloodPlane))
  (bind (_min _max) (Components|StaticMesh|GetLocalBounds _bloodplane_2))
  (bind _returnvalue (Transformation|GetWorldScale _bloodplane_2))
  (bind _returnvalue_2 (Transformation|GetWorldTransform _bloodplane))
  (bind (_min_2 _max_2) (Components|StaticMesh|GetLocalBounds _bloodplane))
  (bind _returnvalue_3 (Math|Transform|InverseTransformLocation _returnvalue_2 WorldLocation))
  (bind _returnvalue_4 (Math|Float|Absolute(Float) (.x _returnvalue)))
  (bind _returnvalue_5 (Math|Float|Absolute(Float) (.y _returnvalue)))
  (bind _returnvalue_6 (- (.x _max) (.x _min)))
  (bind _returnvalue_7 (- (.y _max) (.y _min)))
  (bind _returnvalue_8 (* _returnvalue_4 _returnvalue_6))
  (bind _returnvalue_9 (* _returnvalue_7 _returnvalue_5))
  (bind _returnvalue_10 (/ MopWidth _returnvalue_9))
  (bind _returnvalue_11 (/ MopWidth _returnvalue_8))
  (bind _returnvalue_12 (* _returnvalue_10 512.0))
  (bind _returnvalue_13 (* _returnvalue_11 512.0))
  (if (not (Variables|Default|GetisCompleted))
    (bind (_canvas _size _context) (Rendering|BeginDrawCanvastoRenderTarget (Variables|Default|GetCleanRenderTarget)))
    (Canvas|DrawMaterial :self _canvas :RenderMaterial "/Game/DOC/BloodPuddleLogic/M_CleanBrush.M_CleanBrush" :ScreenPosition (Math|Vector2D|MakeVector2D (- (* (Math|Float|MapRangeClamped (.x _returnvalue_3) (.x _min_2) (.x _max_2) 0.0 1.0) 512.0) (/ _returnvalue_13 2.0)) (- (* (Math|Float|MapRangeClamped (.y _returnvalue_3) (.y _min_2) (.y _max_2) 0.0 1.0) 512.0) (/ _returnvalue_12 2.0))) :ScreenSize (Math|Vector2D|MakeVector2D _returnvalue_13 _returnvalue_12) :CoordinateSize "(X=1.000000,Y=1.000000)" :PivotPoint "(X=0.500000,Y=0.500000)")
    (Rendering|EndDrawCanvastoRenderTarget _context)
    (Variables|Default|SetStepsSinceLastProgressCheck (+ (Variables|Default|GetStepsSinceLastProgressCheck) 1))
    (if (>= (Variables|Default|GetStepsSinceLastProgressCheck) (Variables|Default|GetProgressCheckInterval))
      (Variables|Default|SetStepsSinceLastProgressCheck 0)
      (CallFunction|UpdateCleanProgress))))

(fn MeasureBloodAmmount
  (LocalVariables|SetTotalBlood 0)
  (Rendering|DrawMaterialtoRenderTarget (Variables|Default|GetProgressRenderTarget) (Variables|Default|GetBloodProgressMaterialDynamic))
  (bind _outsamples (Class|KismetRenderingLibrary|ReadRenderTarget (Variables|Default|GetProgressRenderTarget) true))
  (for _array_element _outsamples
    (LocalVariables|SetTotalBlood (+ (.R (Math|Color|BreakColor _array_element)) (LocalVariables|GetTotalBlood))))
  (return (LocalVariables|GetTotalBlood)))

(fn UpdateCleanProgress
  (bind _boodammount (CallFunction|MeasureBloodAmmount))
  (bind _output_get (Variables|Default|SetCurrentBloodAmmount _boodammount))
  (bind _output_get_2 (Variables|Default|SetCleanPercentage (Math|Float|Clamp(Float) (- 1.0 (/ _output_get (Variables|Default|GetInitialBloodAmount))))))
  (if (and (>= _output_get_2 (Variables|Default|GetCompletionThreshold)) (not (Variables|Default|GetisCompleted)))
    (CallFunction|PuddleCleaned)))