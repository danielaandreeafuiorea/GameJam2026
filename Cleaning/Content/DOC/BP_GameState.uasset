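; BP_GameState tracks the current day and its chore counters, such as blood cleaning, skeleton poking and spider killing.
; CheckTasks tests a growing set of counters for each of days one to three and calls NewDay when all in that set equal zero.
; NewDay increments the day and resets every counter to zero.
; Nothing in this graph changes the counters otherwise or calls CheckTasks.
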(event Custom|CheckTasks
  (switch int (Variables|Default|GetDay)
    (:1
      (if (and (== (Variables|Default|GetBlood3DCleaned) 0) (== (Variables|Default|GetBlood2DCleaned) 0))
        (CallFunction|NewDay)))
    (:2
      (if (Math|Boolean|ANDBoolean (== (Variables|Default|GetBlood3DCleaned) 0) (== (Variables|Default|GetBlood2DCleaned) 0) (== (Variables|Default|GetPokedSkeletons) 0) (== (Variables|Default|GetAngryBirds) 0))
        (CallFunction|NewDay)))
    (:3
      (if (Math|Boolean|ANDBoolean (== (Variables|Default|GetBlood3DCleaned) 0) (== (Variables|Default|GetBlood2DCleaned) 0) (== (Variables|Default|GetPokedSkeletons) 0) (== (Variables|Default|GetAngryBirds) 0) (== (Variables|Default|GetSpidersDead) 0) (== (Variables|Default|GetArmourSorted) 0) (== (Variables|Default|GetCockroachCrushed) 0))
        (CallFunction|NewDay)))))

(event Custom|NewDay
  (Math|Integer|IncrementInt (Variables|Default|GetDay)
    (:%20%20
      (Variables|Default|SetBlood3DCleaned 0)
      (Variables|Default|SetBlood2DCleaned 0)
      (Variables|Default|SetPokedSkeletons 0)
      (Variables|Default|SetAngryBirds 0)
      (Variables|Default|SetSpidersDead 0)
      (Variables|Default|SetArmourSorted 0)
      (Variables|Default|SetCockroachCrushed 0))))

(event EventBeginPlay)

(event EventTick
  (params (DeltaSeconds :type Float%20%28single-precision%29)))

(fn ConstructionScript)