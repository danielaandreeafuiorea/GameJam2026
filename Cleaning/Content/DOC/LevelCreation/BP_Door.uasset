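; BP_Door is a trigger doorway that moves the player between rooms through a linked door.
; On BeginPlay it caches the level's camera rig and its parent BP_Room.
; Player overlap asks the rig, unless already transitioning, to start a transition to the linked door's room and entry point, raised by capsule half-height.
; Construction sets trigger size and entry offset, while ConfigureDoor resizes and repositions the trigger from given dimensions.
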(event EventBeginPlay
  (Utilities|FlowControl|Sequence
    (:then_0
      (bind _returnvalue (Actor|GetActorOfClass "/Game/DOC/LevelCreation/BP_CameraRig.BP_CameraRig_C"))
      (bind _asbp_camera_rig (Utilities|Casting|CastToBP_CameraRig _returnvalue))
      (Variables|Default|SetCameraRig _asbp_camera_rig))
    (:then_1
      (bind _asbp_room (Utilities|Casting|CastToBP_Room (Actor|GetParentActor)))
      (Variables|Default|SetOwningRoom _asbp_room))))

(event EventTick
  (params (DeltaSeconds :type Float%20%28single-precision%29)))

(event Collision|EventActorBeginOverlap
  (params (OtherActor :type Actor%20Object%20Reference))
  (bind _linkeddoor (Variables|Default|GetLinkedDoor))
  (bind _entrypoint (Variables|BP_Door_C|GetEntryPoint _linkeddoor))
  (bind _returnvalue (Transformation|GetWorldLocation _entrypoint))
  (Utilities|Casting|CastToBP_Player OtherActor)
  (Utilities|IsValid (Variables|Default|GetLinkedDoor)
    (:Is%20Valid
      (Utilities|IsValid (Variables|Default|GetCameraRig)
        (:Is%20Valid
          (if (not (Variables|/Game/DOC/LevelCreation/BP_CameraRig.BP_CameraRig_C|GetbIsTransitioning (Variables|Default|GetCameraRig)))
            (bind _asbp_player (Utilities|Casting|CastToBP_Player (Game|Player|GetPlayerPawn 0)))
            (Default|StartRoomTransition (Variables|Default|GetCameraRig) (Variables|BP_Door_C|GetOwningRoom _linkeddoor) (Math|Vector|MakeVector (.x _returnvalue) (.y _returnvalue) (+ (.z _returnvalue) (Components|Capsule|GetScaledCapsuleHalfHeight (Variables|/Script/Engine.Character|GetCapsuleComponent _asbp_player)))))))))))

(fn ConstructionScript
  (Components|Box|SetBoxExtent (Variables|Default|GetTrigger) (Math|Vector|MakeVector 7e+01 (/ (Variables|Default|GetDoorWidth) 2.0) 1.5e+02) true)
  (Transformation|SetRelativeLocation (Variables|Default|GetEntryPoint) (Math|Vector|MakeVector (* (Variables|Default|GetEntryOffset) -1.0) 0.0 0.0) false true))

(fn ConfigureDoor
  (params (NewDoorWidth :type Float%20%28double-precision%29) (NewDoorHeight :type Float%20%28double-precision%29) (NewDoorThickness :type Float%20%28double-precision%29))
  (Variables|Default|SetDoorWidth NewDoorWidth)
  (Variables|Default|SetDoorHeigth NewDoorHeight)
  (Variables|Default|SetDoorThickness NewDoorThickness)
  (Components|Box|SetBoxExtent (Variables|Default|GetTrigger) (Math|Vector|MakeVector (/ (Variables|Default|GetDoorThickness) 2.0) (/ (Variables|Default|GetDoorWidth) 2.0) (/ (Variables|Default|GetDoorHeigth) 2.0)) true)
  (Transformation|SetRelativeLocation (Variables|Default|GetTrigger) (Math|Vector|MakeVector 0.0 0.0 (/ (Variables|Default|GetDoorHeigth) 2.0)) false true))