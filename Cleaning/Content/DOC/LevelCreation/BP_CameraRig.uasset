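; BP_CameraRig is the player's view target, a room-based camera that follows the player.
; Each Tick it tracks the player's X and Y, clamped to the current room's CameraBounds box, starting from StartingRoom.
; StartRoomTransition locks move input and cleaning, teleports the player to the destination, and slides the camera there along a timeline.
; When the timeline finishes, it switches rooms, resets the player's last mop position and restores control.
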(event Custom|StartRoomTransition
  (params (NewRoom :type BP%20Room%20Object%20Reference) (DestinationLocation :type Vector))
  (bind _playerref (Variables|Default|GetPlayerRef))
  (bind _playerref_2 (Variables|Default|GetPlayerRef))
  (Variables|Default|SetbIsTransitioning true)
  (Variables|/Game/DOC/BP_Player.BP_Player_C|SetisInTransition _playerref true)
  (Variables|/Game/DOC/BP_Player.BP_Player_C|SetisCleaning _playerref false)
  (Input|SetIgnoreMoveInput (Game|GetPlayerController 0) true)
  (Variables|Default|SetTransitionStartLocation (Transformation|GetActorLocation))
  (Transformation|SetActorLocation (Variables|Default|GetPlayerRef) DestinationLocation false true)
  (Variables|Default|SetTransitionTargetLocation DestinationLocation)
  (Variables|Default|SetPendingRoom NewRoom)
  (bind _alpha (Timeline|TL_RoomTransition PlayFromStart)
    (:Update
      (Transformation|SetActorLocation (Math|Vector|Lerp(Vector) (Variables|Default|GetTransitionStartLocation) (Variables|Default|GetTransitionTargetLocation) _alpha) false true))
    (:Finished
      (Variables|Default|SetCurrentRoom (Variables|Default|GetPendingRoom))
      (Transformation|SetActorLocation (Transformation|GetActorLocation (Variables|Default|GetPlayerRef)) false true)
      (Variables|Default|SetbIsTransitioning false)
      (Variables|/Game/DOC/BP_Player.BP_Player_C|SetisInTransition _playerref_2 false)
      (Variables|/Game/DOC/BP_Player.BP_Player_C|SetLastCleanLocation _playerref_2 (Transformation|GetWorldLocation (Variables|/Game/DOC/BP_Player.BP_Player_C|GetMopPoint _playerref_2)))
      (Input|SetIgnoreMoveInput (Game|GetPlayerController 0) false))))

(event EventBeginPlay
  (bind _asbp_player (Utilities|Casting|CastToBP_Player (Game|Player|GetPlayerPawn 0)))
  (Variables|Default|SetPlayerRef _asbp_player)
  (Variables|Default|SetCurrentRoom (Variables|Default|GetStartingRoom))
  (Transformation|SetActorLocation (Transformation|GetActorLocation (Variables|Default|GetPlayerRef)) false true)
  (Game|Player|SetViewTargetwithBlend (Game|GetPlayerController 0) self 0.0 "VTBlend_Linear" 0.0 false))

(event Collision|EventActorBeginOverlap
  (params (OtherActor :type Actor%20Object%20Reference)))

(event EventTick
  (params (DeltaSeconds :type Float%20%28single-precision%29))
  (bind _currentroom (Variables|Default|GetCurrentRoom))
  (bind _playerref (Variables|Default|GetPlayerRef))
  (bind _returnvalue (Transformation|GetActorLocation _playerref))
  (bind _camerabounds (Variables|/Game/DOC/LevelCreation/BP_Room.BP_Room_C|GetCameraBounds _currentroom))
  (bind _returnvalue_2 (Transformation|GetWorldLocation _camerabounds))
  (bind _returnvalue_3 (Components|Box|GetScaledBoxExtent _camerabounds))
  (if (not (Variables|Default|GetbIsTransitioning))
    (Utilities|IsValid (Variables|Default|GetPlayerRef)
      (:Is%20Valid
        (Transformation|SetActorLocation (Math|Vector|MakeVector (Math|Float|Clamp(Float) (.x _returnvalue) (- (.x _returnvalue_2) (.x _returnvalue_3)) (+ (.x _returnvalue_2) (.x _returnvalue_3))) (Math|Float|Clamp(Float) (.y _returnvalue) (- (.y _returnvalue_2) (.y _returnvalue_3)) (+ (.y _returnvalue_2) (.y _returnvalue_3))) (.z (Transformation|GetActorLocation))) false true)))))

(fn ConstructionScript)